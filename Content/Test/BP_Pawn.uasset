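; BP_Pawn is a test pawn that inspects the bindings of a Level Sequence at runtime.
; On BeginPlay it creates a player for NewLevelSequence, then prints the name of each binding in that sequence.
; Disconnected experiments remain for querying possessables, printing track names, swapping a BP_Pawn skeletal mesh to Dukemon and calling Play, so none of these run.
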(event `self.ReceiveBeginPlay`
  ;[1 1 1] 베이스폰 가져오기
  (bind (_outactor _returnvalue) (`LevelSequencePlayer.CreateLevelSequencePlayer` "/Game/Test/NewLevelSequence.NewLevelSequence"))
  (set `self.LevelSequencePlayer` _returnvalue)
  (bind _output_get (set `self.LevelSequence` _outactor))
  (bind _returnvalue_2 (`MovieSceneSequenceExtensions.GetBindings` (`LevelSequenceActor.GetSequence` _output_get)))
  (for _index (range (`KismetArrayLibrary.Array_Length` _returnvalue_2))
    (bind _returnvalue_3 (`MovieSceneBindingExtensions.GetName` (`|GetArrayItem` _returnvalue_2 _index)))
    (`KismetSystemLibrary.PrintString` _returnvalue_3)))

(fn `UserConstructionScript`)
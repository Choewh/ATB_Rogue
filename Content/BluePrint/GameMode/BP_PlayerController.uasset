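; Player controller that handles Enhanced Input for camera look, boom zoom and cursor-based target picking.
; BeginPlay caches the BP_BasePawn and adds the IMC_Player mapping context.
; Look input drives yaw and pitch, while IA_Mouse_Left adjusts the pawn's spring arm length.
; IA_Mouse_Right traces from the camera to the cursor's impact point with debug drawing and stores the hit in TargetLocation, which is not consumed here.
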(event `self.ReceiveBeginPlay`
  (bind _asbp_base_pawn (cast `/Game/BluePrint/BP_BasePawn` (`GameplayStatics.GetPlayerPawn` 0)))
  (set `self.BasePlayer` _asbp_base_pawn)
  (set `self.TargetLocation` (0.0 0.0 0.0))
  (`EnhancedInputSubsystemInterface.AddMappingContext` (pcsubsystem `EnhancedInputLocalPlayerSubsystem` self) "/Game/BluePrint/Input/IMC_Player.IMC_Player" 0 (struct)))

(event `EnhancedInput|`
  (params (ActionValue :type Boolean) (ElapsedSeconds :type "Float (double-precision)") (TriggeredSeconds :type "Float (double-precision)"))
  (:`Triggered`
    (`self.AddYawInput` ActionValue_X)
    (`self.AddPitchInput` ActionValue_Y)))

(event `EnhancedInput|/Game/BluePrint/Input/IA_Mouse_Left`
  (params (ActionValue :type "Float (double-precision)") (ElapsedSeconds :type "Float (double-precision)") (TriggeredSeconds :type "Float (double-precision)") (InputAction :type "InputAction Object Reference" :default "/Game/BluePrint/Input/IA_Mouse_Left.IA_Mouse_Left"))
  (bind _returnvalue (`self.GetComponentByClass` (`self.BasePlayer`) "/Script/Engine.SpringArmComponent"))
  (:`Triggered`
    (set `SpringArmComponent.TargetArmLength` (+ (`SpringArmComponent.TargetArmLength` _returnvalue) (* ActionValue 20.0)) _returnvalue)))

(event `EnhancedInput|/Game/BluePrint/Input/IA_Mouse_Right`
  (params (ActionValue :type Boolean) (ElapsedSeconds :type "Float (double-precision)") (TriggeredSeconds :type "Float (double-precision)") (InputAction :type "InputAction Object Reference" :default "/Game/BluePrint/Input/IA_Mouse_Right.IA_Mouse_Right"))
  (:`Started`
    (bind _outhit (`KismetSystemLibrary.LineTraceSingleByProfile` :`Start` (`PlayerCameraManager.GetCameraLocation` (`GameplayStatics.GetPlayerCameraManager` 0)) :`End` (`.ImpactPoint` (`GameplayStatics.BreakHitResult` (`self.GetHitResultUnderCursorByChannel` "TraceTypeQuery1"))) :`ProfileName` "BlockAll" :`DrawDebugType` "ForDuration"))
    (set `self.TargetLocation` (`.Location` (`GameplayStatics.BreakHitResult` _outhit)))))

(fn `UserConstructionScript`)
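; Base pawn for what appears to be a turn-based battle with an active-time gauge.
; On BeginPlay it caches the player controller; each Tick, ABTFeeling adds Feel to ABT until it reaches 1000, printing the value.
; MoveTo lerps the pawn a fixed fraction toward the controller's TargetLocation per call.
; EntryBattle is empty, and the BattleSubsystem calls for enemy entry and turn activation are disconnected.
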(event `self.ReceiveBeginPlay`
  (bind _asbp_player_controller (cast `/Game/BluePrint/GameMode/BP_PlayerController` (`GameplayStatics.GetPlayerController` 0)))
  (set `self.PlayerController` _asbp_player_controller))

(event `EntryBattle`)

(event `self.ReceiveTick`
  (params (DeltaSeconds :type "Float (single-precision)"))
  (`self.ABTFeeling`))

(fn `ABTFeeling`
  (if true
    (if (not (>= (`self.ABT_`) 1000.0))
      (bind _output_get (set `self.ABT_` (+ (`self.ABT_`) (`self.Feel`))))
      (`KismetSystemLibrary.PrintString` (`KismetStringLibrary.Conv_DoubleToString` _output_get)))))

(fn `MoveTo`
  (returns (goal :type Boolean))
  (bind (_sweephitresult _returnvalue) (`self.K2_SetActorLocation` (`KismetMathLibrary.VLerp` (`self.K2_GetActorLocation`) (`/Game/BluePrint/GameMode/BP_PlayerController.TargetLocation` (`self.PlayerController`)) 0.2)))
  (if _returnvalue
    _))

(fn `UserConstructionScript`)
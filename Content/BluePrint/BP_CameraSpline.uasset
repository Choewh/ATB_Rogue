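; BP_CameraSpline is a spline camera rig meant to move SplineCamera along a spline, but its logic is disconnected and BeginPlay does nothing.
; The unwired chain calls SetViewTargetWithBlend without a target and plays a Timeline at a rate derived from CompleteTime.
; Timeline updates would map alpha to spline distance, setting world location and local-space roll and pitch, without yaw.
; A separate unwired "SplineCamera" tag lookup leaves its result unused.
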(event `self.ReceiveBeginPlay`)

(fn `UserConstructionScript`)